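; BP_Collector is a Blueprint that counts overlapping BP_Drum and BP_Plank actors against required amounts.
; On overlap, a successful drum cast increments DrumCount, then the same actor is cast to BP_Plank to increment PlankCount.
; Because the casts are chained, the plank count only rises for an actor passing both.
; The final checks compare both counts to RequireDrum and RequirePlank, but nothing follows a match.
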(event EventBeginPlay)

(event EventTick
  (params (DeltaSeconds :type Float%20%28single-precision%29)))

(event Collision|EventActorBeginOverlap
  (params (OtherActor :type Actor%20Object%20Reference))
  (Utilities|Casting|CastToBP_Drum OtherActor)
  (Variables|Default|SetDrumCount (+ (Variables|Default|GetDrumCount) 1))
  (Utilities|Casting|CastToBP_Plank OtherActor)
  (Variables|Default|SetPlankCount (+ (Variables|Default|GetPlankCount) 1))
  (if (== (Variables|Default|GetDrumCount) (Variables|Default|GetRequireDrum))
    (if (== (Variables|Default|GetPlankCount) (Variables|Default|GetRequirePlank))
      _)))

(fn ConstructionScript)